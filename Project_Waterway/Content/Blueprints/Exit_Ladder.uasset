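; Exit ladder actor that lets the player escape the level once they hold the exit key.
; While the player overlaps it, Tick runs a dot-product look check, showing either the escape or need-key prompt and setting ExitLadderValid or updating the HUD's find-key state.
; PlayerEscapes disables input, fades out, plays the hatch sound, flags the win message for Tick to display, then opens a level using the current level object's name.
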(event `self.ReceiveActorBeginOverlap`
  (params (OtherActor :type "Actor Object Reference"))
  ;[0.05127 0.05127 0.05127] Checking if the player is inside the circle or not, and storing that data for later
  (bind _asbp_first_person_character (cast `/Game/Blueprints/Drive/BP_FirstPersonCharacter` OtherActor))
  (set `self.BP_CharacterController` _asbp_first_person_character))

(event `self.ReceiveActorEndOverlap`
  (params (OtherActor :type "Actor Object Reference"))
  ;[0.05127 0.05127 0.05127] Checking if the player is inside the circle or not, and storing that data for later
  (cast `/Game/Blueprints/Drive/BP_FirstPersonCharacter` OtherActor)
  (set `self.BP_CharacterController` null)
  (`Widget.RemoveFromParent` (`self.Widget Ref`))
  (`Widget.RemoveFromParent` (`self.Widget Ref_2`)))

(event `self.ReceiveTick`
  (params (DeltaSeconds :type "Float (single-precision)"))
  (`self.Look Check Ladder`))

(event `Player Escapes`
  ;[0.05127 0.05127 0.05127] Win State
  (`WidgetLayoutLibrary.RemoveAllWidgets`)
  (`TimelineComponent.Stop` (`/Game/Blueprints/Drive/BP_FirstPersonCharacter.Footstep_Timeline` (`self.BP_CharacterController`)))
  (set `self.Player Has Escaped` true)
  (set `/Game/Blueprints/Drive/BP_FirstPersonCharacter.Has Escaped` true (`self.BP_CharacterController`))
  (`self.DisableInput` (`self.BP_CharacterController`) null)
  (`PlayerCameraManager.StartCameraFade` :`self` (`GameplayStatics.GetPlayerCameraManager` 0) :`ToAlpha` 1.0 :`Duration` 1.0 :`bHoldWhenFinished` true)
  (`KismetSystemLibrary.Delay` 2.0)
  (`GameplayStatics.PlaySound2D` "/Game/Audio/ExitHatch/SC_ExitHatchOpen.SC_ExitHatchOpen" 1.0 1.0 0.0 null null)
  (`KismetSystemLibrary.Delay` 3.0)
  (set `self.Show Win Message` true)
  (`KismetSystemLibrary.Delay` 5.0)
  (`GameplayStatics.OpenLevel` (`KismetStringLibrary.Conv_StringToName` (`KismetSystemLibrary.GetObjectName` (`self.GetLevel`)))))

(event `self.ReceiveBeginPlay`
  (bind _returnvalue (`GameplayStatics.GetPlayerController` 0))
  (bind _returnvalue_2 (`|CreateWidget` "/Game/Widgets/Exit_Ladder_Widget.Exit_Ladder_Widget_C" _returnvalue))
  (set `self.Widget Ref` _returnvalue_2)
  (bind _returnvalue_3 (`|CreateWidget` "/Game/Widgets/Exit_Ladder_Need_Key_Widget.Exit_Ladder_Need_Key_Widget_C" _returnvalue))
  (set `self.Widget Ref_2` _returnvalue_3))

(fn `Look Check Ladder`
  ;[1 1 1] Checking if they are near the switch / Checking if they are looking at the switch / showing text on the UI when both are true
  (if (`self.Player Has Escaped`)
    (if (`self.Show Win Message`)
      (bind _returnvalue (`|CreateWidget` "/Game/Widgets/Escaped_Success_Widget.Escaped_Success_Widget_C" (`GameplayStatics.GetPlayerController` 0)))
      (`UserWidget.AddToViewport` _returnvalue 0)
      (else
        (`Widget.RemoveFromParent` (`self.Widget Ref_2`))
        (`Widget.RemoveFromParent` (`self.Widget Ref`))
        (set `/Game/Blueprints/Drive/BP_FirstPersonCharacter.Exit Ladder Valid` false (`self.BP_CharacterController`))))
    (elif (`KismetSystemLibrary.IsValid` (`self.BP_CharacterController`))
      (if (> (`KismetMathLibrary.Dot_VectorVector` (`SceneComponent.GetForwardVector` (`/Game/Blueprints/Drive/BP_FirstPersonCharacter.FirstPersonCamera` (`self.BP_CharacterController`))) (`KismetMathLibrary.Normal` (- (`self.K2_GetActorLocation`) (`self.K2_GetActorLocation` (`self.BP_CharacterController`))))) (`self.Angle Allow`))
        (set `self.Player Looking at Ladder` true)
        (if (`/Game/Blueprints/Drive/BP_FirstPersonCharacter.Has Exit Key` (`self.BP_CharacterController`))
          (`UserWidget.AddToViewport` (`self.Widget Ref`) 0)
          (set `/Game/Blueprints/Drive/BP_FirstPersonCharacter.Exit Ladder Valid` true (`self.BP_CharacterController`))
          (else
            (`UserWidget.AddToViewport` (`self.Widget Ref_2`) 0)
            (bind _asnew_hud (cast `/Game/Blueprints/NewHUD` (`PlayerController.GetHUD` (`GameplayStatics.GetPlayerController` 0))))
            (`/Game/Widgets/HUD_Objective_Widget.Find Exit Key` (`/Game/Blueprints/NewHUD.HUD Widget Ref` _asnew_hud))))
        (else
          (set `self.Player Looking at Ladder` false)
          (`Widget.RemoveFromParent` (`self.Widget Ref`))
          (`Widget.RemoveFromParent` (`self.Widget Ref_2`))
          (set `/Game/Blueprints/Drive/BP_FirstPersonCharacter.Exit Ladder Valid` false (`self.BP_CharacterController`)))))))

(fn `UserConstructionScript`)