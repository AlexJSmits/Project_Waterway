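; Emergency light actor that pulses a point light's intensity over time.
; On BeginPlay, a timeline plays at the PulseSpeed rate and drives the light's intensity from its float track.
; A TurnLightsOff event toggles the point light's visibility and plays the audio component.
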(event `self.ReceiveBeginPlay`
  (`TimelineComponent.SetPlayRate` (`self.Timeline`) (`self.Pulse Speed`))
  (bind (_direction _newtrack_0) (`Timeline|Timeline`)
    (:`Update`
      (`LightComponent.SetIntensity` (`self.PointLight`) _newtrack_0))))

(event `TurnLightsOff`
  (`SceneComponent.ToggleVisibility` (`self.PointLight`) false)
  (`AudioComponent.Play` (`self.Audio`) 0.0))

(fn `UserConstructionScript`)