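; BP_Stalker_V2 is a stalker enemy pawn that positions itself on two distance rings around the player and can kill them.
; Tick derives ring and attack flags from a stored player distance, while a camera dot-product check flags whether the player is looking at it.
; Separately callable events refresh that distance, AI-move to either ring, or chase the player.
; A successful chase disables input, shows the player's jumpscare mesh with camera shake, then reloads the level.
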(event `self.ReceiveTick`
  (params (DeltaSeconds :type "Float (single-precision)"))
  ;[1 1 1] Constantly Check Which Ring the Player is In
  (`|ExecutionSequence`
    (:`then_0`
      (if (< (`self.Distance to Player`) (* (`self.Ring 1 Radius`) 0.5))
        (set `self.Attacking Player` true)
        (else
          (set `self.Attacking Player` false))))
    (:`then_1`
      (if (> (`self.Distance to Player`) (`self.Ring 2 Radius`))
        (set `self.Outside Ring 2` true)
        (else
          (set `self.Outside Ring 2` false))))
    (:`then_2`
      (if (< (`self.Distance to Player`) (`self.Ring 1 Radius`))
        (set `self.Inside Ring 1` true)
        (else
          (set `self.Inside Ring 1` false))))))

(event `Return Ditance to Player`
  ;[1 1 1] Get Distance between Stalker and Player when Called
  (set `self.Distance to Player` (`self.GetDistanceTo` (`GameplayStatics.GetPlayerCharacter` 0))))

(event `self.ReceiveBeginPlay`
  ;[1 1 1] Get Reference to Player on Start
  (bind _asbp_first_person_character (cast `/Game/Blueprints/Drive/BP_FirstPersonCharacter` (`GameplayStatics.GetPlayerCharacter` 0)))
  (set `self.Player Character Reference` _asbp_first_person_character))

(event `Move to Ring 1`
  ;[1 1 1] Move to Ring 1
  (`|AIMoveTo` self (+ (* (`KismetMathLibrary.Normal` (- (`self.K2_GetActorLocation`) (`self.K2_GetActorLocation` (`self.Player Character Reference`)))) (`self.Ring 1 Radius`)) (`self.K2_GetActorLocation` (`self.Player Character Reference`))) null))

(event `Move to Ring 2`
  ;[1 1 1] Move to Ring 2
  (`|AIMoveTo` self (+ (* (`KismetMathLibrary.Normal` (- (`self.K2_GetActorLocation`) (`self.K2_GetActorLocation` (`self.Player Character Reference`)))) (`self.Ring 2 Radius`)) (`self.K2_GetActorLocation` (`self.Player Character Reference`))) null))

(event `Check If Player Is Looking`
  ;[1 1 1] Check to See if the player is looking at the stalker
  (if (> (`KismetMathLibrary.Dot_VectorVector` (`SceneComponent.GetForwardVector` (`/Game/Blueprints/Drive/BP_FirstPersonCharacter.FirstPersonCamera` (`self.Player Character Reference`))) (`KismetMathLibrary.Normal` (- (`self.K2_GetActorLocation`) (`self.K2_GetActorLocation` (`self.Player Character Reference`))))) 0.75)
    (set `self.Player Is Looking at Stalker` true)
    (else
      (set `self.Player Is Looking at Stalker` false))))

(event `Attack`
  ;[1 1 1] Attack the Player
  (`|AIMoveTo` self (0.0 0.0 0.0) (`self.Player Character Reference`)
    (:`OnSuccess`
      (`self.Player Death`))))

(event `Player Death`
  ;[1 1 1] Player Death Behaviour
  (`self.DisableInput` (`self.Player Character Reference`) null)
  (`SceneComponent.SetVisibility` (`self.Mesh`) false true)
  (`SceneComponent.SetVisibility` (`/Game/Blueprints/Drive/BP_FirstPersonCharacter.Stalker Jump Scare Mesh` (`self.Player Character Reference`)) true true)
  (`PlayerController.ClientStartCameraShake` :`self` (`GameplayStatics.GetPlayerController` 0) :`Shake` "/Game/Blueprints/Drive/DeathCameraShake.DeathCameraShake_C")
  (`KismetSystemLibrary.Delay` 3.0)
  (`GameplayStatics.OpenLevel` (`KismetStringLibrary.Conv_StringToName` (`KismetSystemLibrary.GetObjectName` (`self.GetLevel`)))))

(fn `UserConstructionScript`)