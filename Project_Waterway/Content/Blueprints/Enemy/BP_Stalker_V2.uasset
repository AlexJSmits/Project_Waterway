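; Stalker enemy pawn that shadows the first-person player from a ringed distance band, then attacks and kills with a jumpscare and level reload.
; Exposes movement, facing, gaze-check and attack events alongside its AIC_Stalker_V2 controller, switching that controller's state.
; Tick updates ring flags and triggers randomized attack cooldowns.
; Repositioning projects onto the middle ring and snaps to nearby NavMarkers, attacking if none exist; safe zones revert attacks to stalking.
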(event `Attack Cooldown Manager`
  ;[1 1 1] Attack Cooldown Calculation
  (`KismetSystemLibrary.Delay` (`KismetMathLibrary.RandomFloatInRange` 27.0 63.0))
  (set `self.Can Attack` true))

(event `Face the player`
  (bind (_returnvalue_roll _returnvalue_pitch _returnvalue_yaw) (`KismetMathLibrary.BreakRotator` (`KismetMathLibrary.RInterpTo` (`self.K2_GetActorRotation`) (`KismetMathLibrary.FindLookAtRotation` (`self.K2_GetActorLocation`) (`self.K2_GetActorLocation` (`self.Player Character Reference`))) (`GameplayStatics.GetWorldDeltaSeconds`) 20.0)))
  ;[1 1 1] Face the player when stopped
  (`self.K2_SetActorRotation` (`KismetMathLibrary.MakeRotator` 0.0 0.0 _returnvalue_yaw)))

(event `self.ReceiveTick`
  (params (DeltaSeconds :type "Float (single-precision)"))
  ;[1 1 1] Constantly Check Which Ring the Player is In
  (`|ExecutionSequence`
    (:`then_0`
      (if (`self.Can Attack`)
        (goto _label :!via `Reset`)
        (else
          (`/Engine/EditorBlueprintResources/StandardMacros.DoOnce` false :!label _label
            (:`Completed`
              (`self.Attack Cooldown Manager`))))))
    (:`then_1`
      (if (> (`self.Distance to Player`) (`self.Ring 3 Radius`))
        (set `self.Outside Ring 3` true)
        (else
          (set `self.Outside Ring 3` false))))
    (:`then_2`
      (if (< (`self.Distance to Player`) (`self.Ring 1 Radius`))
        (set `self.Inside Ring 1` true)
        (else
          (set `self.Inside Ring 1` false))))))

(event `Return Ditance to Player`
  ;[1 1 1] Get Distance between Stalker and Player when Called
  (bind _output_get (set `self.Distance to Player` (`self.GetDistanceTo` (`GameplayStatics.GetPlayerCharacter` 0))))
  (if (< _output_get (* (`self.Ring 1 Radius`) 0.5))
    (`/Game/Blueprints/Enemy/AI/AIC_Stalker_V2.Set State As Attacking` (`self.AIC Reference`))))

(event `self.ReceiveBeginPlay`
  ;[1 1 1] Get Reference to Player on Start
  (`KismetSystemLibrary.Delay` 0.1)
  (bind _asbp_first_person_character (cast `/Game/Blueprints/Drive/BP_FirstPersonCharacter` (`GameplayStatics.GetPlayerCharacter` 0)))
  (set `self.Player Character Reference` _asbp_first_person_character)
  (bind _asaic_stalker_v2 (cast `/Game/Blueprints/Enemy/AI/AIC_Stalker_V2` (`AIBlueprintHelperLibrary.GetAIController` self)))
  (set `self.AIC Reference` _asaic_stalker_v2))

(event `Move to Stalking Zone`
  ;[1 1 1] Move the Stalker back into the center of the stalking zone
  (bind _output_get (set `self.Target Destination` (+ (* (`KismetMathLibrary.Normal` (- (`self.K2_GetActorLocation`) (`self.K2_GetActorLocation` (`self.Player Character Reference`)))) (`self.Ring 2 Radius`)) (`self.K2_GetActorLocation` (`self.Player Character Reference`)))))
  (bind _outactors (`KismetSystemLibrary.SphereOverlapActors` _output_get 4000.0 (`|MakeArray` "ObjectTypeQuery2" :!type "EObjectTypeQuery Enum") "/Game/Blueprints/Level_Modules/NavMarker.NavMarker_C"))
  (if (`KismetArrayLibrary.Array_IsValidIndex` _outactors)
    (`|AIMoveTo` self (`self.K2_GetActorLocation` (`.ReturnValue` (`GameplayStatics.FindNearestActor` (`self.Target Destination`) _outactors))) null)
    (else
      (`/Game/Blueprints/Enemy/AI/AIC_Stalker_V2.Set State As Attacking` (`self.AIC Reference`)))))

(event `Check If Player Is Looking`
  ;[1 1 1] Check to See if the player is looking at the stalker
  (if (> (`KismetMathLibrary.Dot_VectorVector` (`SceneComponent.GetForwardVector` (`/Game/Blueprints/Drive/BP_FirstPersonCharacter.FirstPersonCamera` (`self.Player Character Reference`))) (`KismetMathLibrary.Normal` (- (`self.K2_GetActorLocation`) (`self.K2_GetActorLocation` (`self.Player Character Reference`))))) 0.75)
    (set `self.Player Is Looking at Stalker` true)
    (else
      (set `self.Player Is Looking at Stalker` false))))

(event `Attack`
  ;[1 1 1] Attack the Player
  (if (`/Game/Blueprints/Drive/BP_FirstPersonCharacter.Inside Safe Zone` (`self.Player Character Reference`))
    (`/Game/Blueprints/Enemy/AI/AIC_Stalker_V2.Set State As Stalking` (`self.AIC Reference`))
    (else
      (`AIController.K2_SetFocus` (`self.AIC Reference`) null)
      (`|AIMoveTo` self (0.0 0.0 0.0) (`self.Player Character Reference`)
        (:`OnSuccess`
          (`/Engine/EditorBlueprintResources/StandardMacros.DoOnce` false
            (:`Completed`
              (`self.Player Death`))))))))

(event `Player Death`
  (bind _player_character_reference (`self.Player Character Reference`))
  ;[1 1 1] Player Death Behaviour
  (`GameplayStatics.PlaySound2D` "/Game/Audio/Enemy/SC_PlayerDeath.SC_PlayerDeath" 1.0 1.0 0.0 null null)
  (if (not (`/Game/Blueprints/Drive/BP_FirstPersonCharacter.Has Escaped` _player_character_reference))
    (`self.DisableInput` _player_character_reference null)
    (`SkeletalMeshComponent.Play` (`/Game/Blueprints/Drive/BP_FirstPersonCharacter.Stalker Jump Scare Mesh` (`self.Player Character Reference`)) false)
    (`SceneComponent.SetVisibility` (`self.Mesh`) false true)
    (`SceneComponent.SetVisibility` (`/Game/Blueprints/Drive/BP_FirstPersonCharacter.Stalker Jump Scare Mesh` (`self.Player Character Reference`)) true true)
    (`PlayerController.ClientStartCameraShake` :`self` (`GameplayStatics.GetPlayerController` 0) :`Shake` "/Game/Blueprints/Drive/DeathCameraShake.DeathCameraShake_C")
    (`KismetSystemLibrary.Delay` 3.0)
    (`GameplayStatics.OpenLevel` (`KismetStringLibrary.Conv_StringToName` (`KismetSystemLibrary.GetObjectName` (`self.GetLevel`))))))

(event `Check Left`
  (bind (_returnvalue_x _returnvalue_y _returnvalue_z) (`KismetMathLibrary.BreakVector` (`self.K2_GetActorLocation` (`self.Player Character Reference`))))
  ;[1 1 1] Move the Stalker back into the center of the stalking zone
  (bind _output_get (set `self.Target Destination` (+ (* (`KismetMathLibrary.Normal` (- (`self.K2_GetActorLocation`) (`self.K2_GetActorLocation` (`self.Player Character Reference`)))) (`self.Ring 2 Radius`)) (`KismetMathLibrary.MakeVector` _returnvalue_x (+ _returnvalue_y 4000.0) _returnvalue_z))))
  (bind _outactors (`KismetSystemLibrary.SphereOverlapActors` _output_get 4000.0 (`|MakeArray` "ObjectTypeQuery2" :!type "EObjectTypeQuery Enum") "/Game/Blueprints/Level_Modules/NavMarker.NavMarker_C"))
  (if (`KismetArrayLibrary.Array_IsValidIndex` _outactors)
    (`|AIMoveTo` self (`self.K2_GetActorLocation` (`.ReturnValue` (`GameplayStatics.FindNearestActor` (`self.Target Destination`) _outactors))) null)
    (else
      (`/Game/Blueprints/Enemy/AI/AIC_Stalker_V2.Set State As Attacking` (`self.AIC Reference`)))))

(fn `UserConstructionScript`)