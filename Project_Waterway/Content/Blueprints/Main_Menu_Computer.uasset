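; Main menu laptop actor that serves as the game's start screen, framing the player's first-person camera at a set position.
; The first key press plays a password sound, briefly shows a widget, then timeline-lerps the camera to the laptop view.
; It then opens the Laptop_Screen UI with mouse input and passes itself as reference.
; StartGame animates the widget's game image padding, removes it and loads Waterway_Start.
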(event `Key|AnyKey`
  (params (Key :type "Key Structure"))
  (bind _firstpersoncamera (`/Game/Blueprints/Main_Menu/BP_MainMenuCharacter.FirstPersonCamera` (`self.BP Main Menu Character Reference`)))
  ;[1 1 1] Start Game Button Plressed
  (:`Pressed`
    (`/Engine/EditorBlueprintResources/StandardMacros.DoOnce` false
      (:`Completed`
        (`GameplayStatics.PlaySound2D` "/Game/Audio/Player/CorrectPassword.CorrectPassword" 1.0 1.0 0.0 null null)
        (`SceneComponent.SetVisibility` (`self.Widget`) true false)
        (`KismetSystemLibrary.Delay` 2.0)
        (`SceneComponent.SetVisibility` (`self.Widget`) false false)
        (`KismetSystemLibrary.Delay` 1.0)
        (bind _output_get (set `self.Temp Camera Position` (`SceneComponent.K2_GetComponentToWorld` _firstpersoncamera)))
        (bind (_direction _output) (`Timeline|Timeline_0` :!via `PlayFromStart`)
          (:`Update`
            (`SceneComponent.K2_SetWorldTransform` _firstpersoncamera (`KismetMathLibrary.TLerp` _output_get (`SceneComponent.K2_GetComponentToWorld` (`self.Camera Position Game Start`)) _output) false false))
          (:`Finished`
            (`KismetSystemLibrary.Delay` 0.5)
            (`self.Turn On Laptop`)))))))

(event `Turn On Laptop`
  (bind _returnvalue (`GameplayStatics.GetPlayerController` 0))
  ;[1 1 1] Adds Laptop
  (bind _returnvalue_2 (`|CreateWidget` "/Game/Widgets/Laptop_Screen.Laptop_Screen_C" (`GameplayStatics.GetPlayerController` 0)))
  (bind _output_get (set `self.Laptop Screen Widget` _returnvalue_2))
  (`UserWidget.AddToViewport` _output_get 0)
  (`WidgetBlueprintLibrary.SetInputMode_UIOnlyEx` _returnvalue (`self.Laptop Screen Widget`))
  (set `PlayerController.bShowMouseCursor` true _returnvalue)
  (set `/Game/Widgets/Laptop_Screen.Laptop Reference` self (`self.Laptop Screen Widget`)))

(event `self.ReceiveBeginPlay`
  ;[1 1 1] Comment
  (`KismetSystemLibrary.Delay` 0.1)
  (bind _asbp_main_menu_character (cast `/Game/Blueprints/Main_Menu/BP_MainMenuCharacter` (`GameplayStatics.GetPlayerCharacter` 0)))
  (set `self.BP Main Menu Character Reference` _asbp_main_menu_character)
  (`SceneComponent.K2_SetWorldTransform` (`/Game/Blueprints/Main_Menu/BP_MainMenuCharacter.FirstPersonCamera` (`self.BP Main Menu Character Reference`)) (`SceneComponent.K2_GetComponentToWorld` (`self.Camera Position`)) false false))

(event `Start Game`
  (bind (_intended_padding_left _intended_padding_top _intended_padding_right _intended_padding_bottom) (break `Margin` (`self.Intended Padding`)))
  (bind _returnvalue (`WidgetLayoutLibrary.SlotAsOverlaySlot` (`/Game/Widgets/Laptop_Screen.GameImage` (`self.Laptop Screen Widget`))))
  ;[1 1 1] Start Game Button Plressed
  (bind _output_get (set `self.Current Padding` (`OverlaySlot.Padding` _returnvalue)))
  (bind (_direction _output) (`Timeline|Timeline` :!via `PlayFromStart`)
    (:`Update`
      (`OverlaySlot.SetPadding` _returnvalue (make `Margin` (`KismetMathLibrary.Lerp` (break `Margin` _output_get) _intended_padding_left _output) (`KismetMathLibrary.Lerp` (`.Top` (break `Margin` _output_get)) _intended_padding_top _output) (`KismetMathLibrary.Lerp` (`.Right` (break `Margin` _output_get)) _intended_padding_right _output) (`KismetMathLibrary.Lerp` (`.Bottom` (break `Margin` _output_get)) _intended_padding_bottom _output))))
    (:`Finished`
      (`KismetSystemLibrary.Delay` 1.0)
      (`Widget.RemoveFromParent` (`self.Laptop Screen Widget`))
      (`KismetSystemLibrary.Delay` 2.0)
      (`GameplayStatics.OpenLevel` "Waterway_Start"))))

(fn `UserConstructionScript`)