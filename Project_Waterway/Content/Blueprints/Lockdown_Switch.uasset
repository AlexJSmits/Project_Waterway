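; Lockdown switch actor that shows a power switch prompt when the first-person character is within its overlap area and looking at it.
; Overlap events store the character, and a per-tick dot-product check against AngleAllow sets PlayerLookingAtObject, creating a new widget each passing frame.
; Failed look checks, leaving the area or inactivity clear all widgets.
; SwitchPulled plays a sequence, then after a delay hides the point light and deactivates the switch.
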(event `self.ReceiveActorBeginOverlap`
  (params (OtherActor :type "Actor Object Reference"))
  ;[0.05127 0.05127 0.05127] Checking if the player is inside the circle or not, and storing that data for later
  (bind _asbp_first_person_character (cast `/Game/Blueprints/Drive/BP_FirstPersonCharacter` OtherActor))
  (set `self.BP_CharacterController` _asbp_first_person_character))

(event `self.ReceiveActorEndOverlap`
  (params (OtherActor :type "Actor Object Reference"))
  ;[0.05127 0.05127 0.05127] Checking if the player is inside the circle or not, and storing that data for later
  (cast `/Game/Blueprints/Drive/BP_FirstPersonCharacter` OtherActor)
  (set `self.BP_CharacterController` null)
  (`WidgetLayoutLibrary.RemoveAllWidgets`))

(event `self.ReceiveTick`
  (params (DeltaSeconds :type "Float (single-precision)"))
  (`self.LookCheck`))

(event `Switch Pulled`
  (`ActorSequenceComponent.PlaySequence` (`self.ActorSequence`))
  (`KismetSystemLibrary.Delay` 3.0)
  (`SceneComponent.ToggleVisibility` (`self.PointLight`) false)
  (set `self.Is Active` false))

(fn `LookCheck`
  ;[1 1 1] Checking if they are near the switch / Checking if they are looking at the switch / showing text on the UI when both are true
  (if (`self.Is Active`)
    (if (`KismetSystemLibrary.IsValid` (`self.BP_CharacterController`))
      (if (> (`KismetMathLibrary.Dot_VectorVector` (`SceneComponent.GetForwardVector` (`/Game/Blueprints/Drive/BP_FirstPersonCharacter.FirstPersonCamera` (`self.BP_CharacterController`))) (`KismetMathLibrary.Normal` (- (`self.K2_GetActorLocation`) (`self.K2_GetActorLocation` (`self.BP_CharacterController`))))) (`self.Angle Allow`))
        (set `self.Player Looking at Object` true)
        (bind _returnvalue (`|CreateWidget` "/Game/Widgets/Power_Switch_Widget.Power_Switch_Widget_C" (`GameplayStatics.GetPlayerController` 0)))
        (`UserWidget.AddToViewport` _returnvalue 0)
        (else
          (set `self.Player Looking at Object` false)
          (`WidgetLayoutLibrary.RemoveAllWidgets`))))
    (else
      (`WidgetLayoutLibrary.RemoveAllWidgets`)
      (set `self.Player Looking at Object` false))))

(fn `UserConstructionScript`)