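; Exit key pickup that the first-person character can collect when close to it and looking toward it.
; A sphere overlap stores the character, and a per-tick dot product of camera forward against direction to the key toggles the prompt widget and the character's ExitKeyValid flag.
; PickupKey grants HasExitKey, deactivates and hides the key, then tells the HUD to show the key and lifted emergency lock.
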(event `self.Collider_Sphere.OnComponentBeginOverlap`
  (params (OverlappedComponent :type "PrimitiveComponent Object Reference") (OtherActor :type "Actor Object Reference") (OtherComp :type "PrimitiveComponent Object Reference") (OtherBodyIndex :type Integer) (bFromSweep :type Boolean) (SweepResult :type "HitResult Structure (by ref)"))
  ;[0.05127 0.05127 0.05127] Checking if the player is inside the circle or not, and storing that data for later
  (bind _asbp_first_person_character (cast `/Game/Blueprints/Drive/BP_FirstPersonCharacter` OtherActor))
  (set `self.BP_CharacterController` _asbp_first_person_character))

(event `self.Collider_Sphere.OnComponentEndOverlap`
  (params (OverlappedComponent :type "PrimitiveComponent Object Reference") (OtherActor :type "Actor Object Reference") (OtherComp :type "PrimitiveComponent Object Reference") (OtherBodyIndex :type Integer))
  ;[0.05127 0.05127 0.05127] Checking if the player is inside the circle or not, and storing that data for later
  (cast `/Game/Blueprints/Drive/BP_FirstPersonCharacter` OtherActor)
  (set `self.BP_CharacterController` null)
  (`Widget.RemoveFromParent` (`self.Exit Key Widget Reference`)))

(event `self.ReceiveTick`
  (params (DeltaSeconds :type "Float (single-precision)"))
  (`self.LookCheck`))

(event `self.ReceiveBeginPlay`
  (bind _returnvalue (`|CreateWidget` "/Game/Widgets/Exit_Key_Widget.Exit_Key_Widget_C" (`GameplayStatics.GetPlayerController` 0)))
  (set `self.Exit Key Widget Reference` _returnvalue))

(event `Pickup Key`
  (set `/Game/Blueprints/Drive/BP_FirstPersonCharacter.Has Exit Key` true (`self.BP_CharacterController`))
  (set `self.Is Active` false)
  (`SceneComponent.SetHiddenInGame` (`self.Key`) true true)
  (bind _asnew_hud (cast `/Game/Blueprints/NewHUD` (`PlayerController.GetHUD` (`GameplayStatics.GetPlayerController` 0))))
  (bind _hud_widget_ref (`/Game/Blueprints/NewHUD.HUD Widget Ref` _asnew_hud))
  (`/Game/Widgets/HUD_Objective_Widget.Emegency Lock Lifted` _hud_widget_ref)
  (`/Game/Widgets/HUD_Objective_Widget.Show Key` _hud_widget_ref))

(fn `LookCheck`
  ;[1 1 1] Checking if they are near the switch / Checking if they are looking at the switch / showing text on the UI when both are true
  (if (`self.Is Active`)
    (if (`KismetSystemLibrary.IsValid` (`self.BP_CharacterController`))
      (if (> (`KismetMathLibrary.Dot_VectorVector` (`SceneComponent.GetForwardVector` (`/Game/Blueprints/Drive/BP_FirstPersonCharacter.FirstPersonCamera` (`self.BP_CharacterController`))) (`KismetMathLibrary.Normal` (- (`self.K2_GetActorLocation`) (`self.K2_GetActorLocation` (`self.BP_CharacterController`))))) (`self.Angle Allow`))
        (set `self.Player Looking at Object` true)
        (`UserWidget.AddToViewport` (`self.Exit Key Widget Reference`) 0)
        (set `/Game/Blueprints/Drive/BP_FirstPersonCharacter.Exit Key Valid` true (`self.BP_CharacterController`))
        (else
          (set `self.Player Looking at Object` false)
          (`Widget.RemoveFromParent` (`self.Exit Key Widget Reference`))
          (set `/Game/Blueprints/Drive/BP_FirstPersonCharacter.Exit Key Valid` false (`self.BP_CharacterController`)))))
    (else
      (`Widget.RemoveFromParent` (`self.Exit Key Widget Reference`))
      (set `self.Player Looking at Object` false)
      (set `/Game/Blueprints/Drive/BP_FirstPersonCharacter.Exit Key Valid` false (`self.BP_CharacterController`)))))

(fn `UserConstructionScript`)