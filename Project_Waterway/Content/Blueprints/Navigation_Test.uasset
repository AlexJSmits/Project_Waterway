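; Navigation test pawn that, on BeginPlay, caches the first-person player and runs a single AI move test.
; It computes a point at a fixed distance from the player toward its own position and draws a debug sphere there.
; A sphere overlap around that point looks for NavMarker pawns, and AIMoveTo heads to the point only if at least two are found.
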(event `self.ReceiveBeginPlay`
  ;[1 1 1] Get Reference to Player on Start
  (bind _asbp_first_person_character (cast `/Game/Blueprints/Drive/BP_FirstPersonCharacter` (`GameplayStatics.GetPlayerCharacter` 0)))
  (set `self.Player Character Reference` _asbp_first_person_character)
  (`self.Nav Test`))

(event `Nav Test`
  (bind _returnvalue (+ (* (`KismetMathLibrary.Normal` (- (`self.K2_GetActorLocation`) (`self.K2_GetActorLocation` (`self.Player Character Reference`)))) 1000.0) (`self.K2_GetActorLocation` (`self.Player Character Reference`))))
  ;[1 1 1] Test Navigation
  (`KismetSystemLibrary.DrawDebugSphere` _returnvalue 100.0 12 (struct :`R` 1.0 :`G` 1.0 :`B` 1.0 :`A` 1.0) 10.0 1.0)
  (bind _outactors (`KismetSystemLibrary.SphereOverlapActors` _returnvalue 5000.0 (`|MakeArray` "ObjectTypeQuery3" :!type "EObjectTypeQuery Enum") "/Game/Blueprints/Level_Modules/NavMarker.NavMarker_C"))
  (if (`KismetArrayLibrary.Array_IsValidIndex` _outactors 1)
    (`|AIMoveTo` self _returnvalue null)))

(fn `UserConstructionScript`)